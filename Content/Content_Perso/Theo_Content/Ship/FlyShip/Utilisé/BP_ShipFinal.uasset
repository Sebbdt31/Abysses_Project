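; BP_ShipFinal is a player-controlled ship, driven by physics forces on its shell mesh.
; Forward and right axis inputs add acceleration along the actor's axes, while turn input yaws the controller in proportion to speed.
; Tick computes that speed in knots from velocity and spins the propeller mesh.
; Boarding and exit logic for BP_Eve is disconnected: trigger overlaps are empty and the possession swap never runs.
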(event OnComponentBeginOverlap(Triggerdupilotagebateau)
  (params (OverlappedComponent :type Primitive%20Component%20Object%20Reference) (OtherActor :type Actor%20Object%20Reference) (OtherComp :type Primitive%20Component%20Object%20Reference) (OtherBodyIndex :type Integer) (bFromSweep :type Boolean) (SweepResult :type Hit%20Result%20Structure%20%28by%20ref%29))
  ;[1 1 1] Possession du bateau
)

(event OnComponentEndOverlap(Triggerdupilotagebateau)
  (params (OverlappedComponent :type Primitive%20Component%20Object%20Reference) (OtherActor :type Actor%20Object%20Reference) (OtherComp :type Primitive%20Component%20Object%20Reference) (OtherBodyIndex :type Integer))
  ;[1 1 1] Possession du bateau
)

(event EventTick
  (params (DeltaSeconds :type Float%20%28single-precision%29))
  ;[0 1 0.8237 1 42] Comportement du navire
  ;;[1 1 1 1 30] Recuperer la speed
  (Variables|Default|Setvitesse (Math|Float|Round (* (Math|Vector|VectorLength (Transformation|GetVelocity)) 0.01944)))
  ;[1 1 1] Propeller rotation
  (Transformation|AddLocalRotation (Variables|Default|GetSK_Propeller) "20.000000,0.000000,0.000000" false false))

(event Input|AxisEvents|InputAxisMoveRight
  (params (AxisValue :type Float%20%28single-precision%29))
  ;[0 1 0.8237 1 42] Comportement du navire
  ;;[0 1 0.7117 1 30] Move fwd/aft
  (Physics|AddForce (Variables|Default|GetSM_Shell) (* (Transformation|GetActorRightVector) (* AxisValue 9e+02)) "None" true))

(event Input|AxisEvents|InputAxisMoveForward
  (params (AxisValue :type Float%20%28single-precision%29))
  ;[0 1 0.8237 1 42] Comportement du navire
  ;;[0 1 0.7261 1 30] Move right/left
  (Physics|AddForce (Variables|Default|GetSM_Shell) (* (Transformation|GetActorForwardVector) (* AxisValue 2.5e+02)) "None" true))

(event Input|AxisEvents|InputAxisTurn
  (params (AxisValue :type Float%20%28single-precision%29))
  ;[0 1 0.8237 1 42] Comportement du navire
  ;;[0 1 0.7096 1 30] Yaw Move
  (Pawn|Input|AddControllerYawInput (/ (* AxisValue (Variables|Default|Getvitesse)) 2.5e+02)))

(event Input|KeyboardEvents|E
  (params (Key :type Key%20Structure :default "None"))
  ;[1 1 1] Possession du bateau
)

(fn ConstructionScript)