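; Pilotable boat pawn driven by physics, which the player can board from a trigger zone and leave with E.
; Move axes push the boat mesh with forward and lateral forces, while turn input adds controller yaw scaled by speed, computed each tick in knots.
; The trigger hands the overlapping actor a boat reference and nearby flag; E moves the stored character to the pilot spawn, restores visibility and collision, and repossesses it.
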(event OnComponentBeginOverlap(Triggerdupilotagebateau)
  (params (OverlappedComponent :type Primitive%20Component%20Object%20Reference) (OtherActor :type Actor%20Object%20Reference) (OtherComp :type Primitive%20Component%20Object%20Reference) (OtherBodyIndex :type Integer) (bFromSweep :type Boolean) (SweepResult :type Hit%20Result%20Structure%20%28by%20ref%29))
  ;[1 1 1] Possession du bateau
  (bind _asfirst_person_character (Utilities|Casting|CastTo OtherActor))
  (Variables|Default|Setnear%20boat _asfirst_person_character true)
  (Variables|Default|SetBP_Boat _asfirst_person_character self)
  (Development|PrintString "E"))

(event OnComponentEndOverlap(Triggerdupilotagebateau)
  (params (OverlappedComponent :type Primitive%20Component%20Object%20Reference) (OtherActor :type Actor%20Object%20Reference) (OtherComp :type Primitive%20Component%20Object%20Reference) (OtherBodyIndex :type Integer))
  ;[1 1 1] Possession du bateau
  (bind _asfirst_person_character (Utilities|Casting|CastTo OtherActor))
  (Variables|Default|Setnear%20boat _asfirst_person_character false))

(event EventTick
  (params (DeltaSeconds :type Float%20%28single-precision%29))
  ;[1 1 1 1 30] Recuperer la speed
  (Variables|Default|Setvitesse (Math|Float|Round (* (Math|Vector|VectorLength (Transformation|GetVelocity)) 0.01944))))

(event Input|AxisEvents|InputAxisMoveForward
  (params (AxisValue :type Float%20%28single-precision%29))
  ;[0 1 0.8237 1 42] Comportement du navire
  ;;[0 1 0.7261 1 30] Move fwd/aft
  (Physics|AddForce (Variables|Default|GetSM_boat) (* (Transformation|GetActorForwardVector) (* AxisValue 1.8e+03)) "None" true))

(event Input|AxisEvents|InputAxisMoveRight
  (params (AxisValue :type Float%20%28single-precision%29))
  ;[0 1 0.8237 1 42] Comportement du navire
  ;;[0 1 0.7117 1 30] Move right/left
  (Physics|AddForce (Variables|Default|GetSM_boat) (* (Transformation|GetActorRightVector) (* AxisValue 2.5e+02)) "None" true))

(event Input|AxisEvents|InputAxisTurn
  (params (AxisValue :type Float%20%28single-precision%29))
  ;[0 1 0.8237 1 42] Comportement du navire
  ;;[0 1 0.7096 1 30] Yaw Move
  (Pawn|Input|AddControllerYawInput (/ (* AxisValue (Variables|Default|Getvitesse)) 2.5e+02)))

(event Input|KeyboardEvents|E
  (params (Key :type Key%20Structure))
  (bind _spawn_du_pilote (Variables|Default|GetSpawn%20du%20pilote))
  (bind _character (Variables|Default|GetCharacter))
  (bind _returnvalue (Transformation|GetWorldTransform _spawn_du_pilote))
  (bind (_location _rotation) (Math|Transform|BreakTransform _returnvalue))
  ;[1 1 1] Possession du bateau
  (:Pressed
    (Transformation|SetActorTransform _character (Math|Transform|MakeTransform _location (Math|Rotator|MakeRotator 0.0 0.0 (.Yaw (Math|Rotator|BreakRotator _rotation)))))
    (Rendering|SetActorHiddenInGame _character false)
    (Collision|SetActorEnableCollision _character true)
    (Pawn|Possess (Game|GetPlayerController 0) _character)))

(fn ConstructionScript)